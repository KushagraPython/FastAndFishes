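; Drivable drift car pawn for the R-Tune V2 vehicle system, with manual shifting, air control, interior/chase camera toggle and handbrake-triggered drifting.
; Holding Handbrake sets DriftMode, whose macro runs on AsyncTick to interpolate tire lateral forces and drift torque between drift and base values.
; Tick fakes counter-steer on animated front suspensions, separate from the physics ones, while adjusting rear wheel spin, camera lag and brake lights.
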(event EventTick
  (params (DeltaSeconds :type Float%20%28single-precision%29))
  (Variables|Drift|SetDelta%20Time DeltaSeconds)
  (Rendering|Material|SetScalarParameterValueonMaterials (Variables|Default|GetCoreMesh) "Tail Light Input" (Math|Float|SelectFloat 1.0 0.0 (> (Class|RTuneVehicle|GetBrakesInput) 0.1)))
  ;[1 1 1] Extending the system for counter steer drifting
  (bind _output_get (Variables|Drift|SetAnim%20Steering%20Angle (Math|Float|SelectFloat (* (Variables|Settings|GetDrift%20Max%20Angle) -1.0) (Variables|Settings|GetBase%20Wheel%20Steer%20Angle) (and (Variables|Drift|GetDrift%20Mode) (> (Class|RTuneVehicle|GetSpeedKPH) 0.0)))))
  (bind _output_get_2 (Variables|/Script/RTune.SuspensionComponent|SetMaxSteeringAngle (Variables|Default|GetSuspension%20FR_Anim) _output_get))
  (Variables|/Script/RTune.SuspensionComponent|SetMaxSteeringAngle (Variables|Default|GetSuspension%20FL_Anim) _output_get_2)
  (bind _output_get_3 (Variables|/Script/RTune.SuspensionComponent|SetWheelAngularVelocityMultiplier (Variables|Default|GetSuspension%20RL) (Math|Float|SelectFloat (Math|Float|Lerp 1.0 3.0 (Class|RTuneVehicle|GetThrottleInput)) 1.0 (Variables|Drift|GetDrift%20Mode))))
  (Variables|/Script/RTune.SuspensionComponent|SetWheelAngularVelocityMultiplier (Variables|Default|GetSuspension%20RR) _output_get_3)
  (bind _output_get_4 (Variables|Drift|SetCamera%20Lag (Math|Interpolation|FInterpTo (Variables|Drift|GetCamera%20Lag) (Math|Float|SelectFloat 2.0 1e+01 (Variables|Drift|GetDrift%20Mode)) (Variables|Drift|GetDelta%20Time) 5.0)))
  (Variables|/Script/Engine.SpringArmComponent|SetCameraRotationLagSpeed (Variables|Default|GetSpringArm) _output_get_4)
  (Variables|/Script/RTune.RTuneInteriorComponent|SetbInvert (Variables|Default|GetSteering%20Wheel) (Variables|Drift|GetDrift%20Mode)))

(event EventAsyncTick
  (params (DeltaTime :type Float%20%28single-precision%29))
  ;[0 0 0] This is an example of how the vehicle behaviour can be extended for more complex and intricate behaviour. The inputs here override their original properties. Then the handbrake is pressed, the new lateral force and drift values, and when it is released the base values are used.
  (Variables|Drift|SetAsync%20Time DeltaTime)
  (Utilities|DriftMode 2.5e+02 325.0 3e+03 6.5e+03 5.0 0.0 4e+03))

(event EventBeginPlay
  ;[1 1 1] Initialize suspension array for DriftMode Macro
  (Variables|Drift|SetSuspension (Utilities|Array|MakeArray (Variables|Default|GetPhysisc%20FL) (Variables|Default|GetSuspension%20RR) (Variables|Default|GetSuspension%20RL) (Variables|Default|GetPhysics%20FR))))

(event Input|ActionEvents|InputActionUpshift
  (params (Key :type Key%20Structure :default "None"))
  ;[1 1 1] Input
  (:Pressed
    (if (!= (Variables|Default|GetbAutomatic) true)
      (Class|RTuneVehicle|Upshift))))

(event Input|ActionEvents|InputActionDownshift
  (params (Key :type Key%20Structure :default "None"))
  ;[1 1 1] Input
  (:Pressed
    (if (!= (Variables|Default|GetbAutomatic) true)
      (Class|RTuneVehicle|Downshift))))

(event Input|ActionEvents|InputActionHandbrake
  (params (Key :type Key%20Structure :default "None"))
  ;[1 1 1] Input
  (:Pressed
    (Variables|Drift|SetDrift%20Mode true))
  (:Released
    (Variables|Drift|SetDrift%20Mode false)))

(event Input|ActionEvents|InputActionToggleFreeCamera
  (params (Key :type Key%20Structure :default "None"))
  (bind _springarm (Variables|Default|GetSpringArm))
  ;[1 1 1] Input
  (:Pressed
    (Variables|/Script/Engine.SpringArmComponent|SetbUsePawnControlRotation _springarm (!= (Variables|/Script/Engine.SpringArmComponent|GetbUsePawnControlRotation _springarm) true))))

(event Input|ActionEvents|InputActionToggleCamera
  (params (Key :type Key%20Structure :default "None"))
  ;[1 1 1] Input
  (:Pressed
    (Utilities|FlowControl|FlipFlop
      (:A
        (Components|Activation|SetActive (Variables|Default|GetCamera%20Interior) true false)
        (Components|Activation|SetActive (Variables|Default|GetCamera) false false))
      (:B
        (Components|Activation|SetActive (Variables|Default|GetCamera%20Interior) false false)
        (Components|Activation|SetActive (Variables|Default|GetCamera) true false)))))

(event Input|AxisEvents|InputAxisThrottle
  (params (AxisValue :type Float%20%28single-precision%29))
  ;[1 1 1] Input
  (Class|RTuneVehicle|SetThrottleInput AxisValue))

(event Input|AxisEvents|InputAxisCy
  (params (AxisValue :type Float%20%28single-precision%29))
  ;[1 1 1] Input
  (Pawn|Input|AddControllerPitchInput AxisValue))

(event Input|AxisEvents|InputAxisSteering
  (params (AxisValue :type Float%20%28single-precision%29))
  ;[1 1 1] Input
  (Class|RTuneVehicle|SetSteeringInput AxisValue))

(event Input|AxisEvents|InputAxisCx
  (params (AxisValue :type Float%20%28single-precision%29))
  ;[1 1 1] Input
  (Pawn|Input|AddControllerYawInput AxisValue))

(event Input|AxisEvents|InputAxisBrake
  (params (AxisValue :type Float%20%28single-precision%29))
  ;[1 1 1] Input
  (Class|RTuneVehicle|SetBrakeInput AxisValue))

(event Input|AxisEvents|InputAxisAirPitch
  (params (AxisValue :type Float%20%28single-precision%29))
  ;[1 1 1] Input
  (Class|RTuneVehicle|SetAirPitchInput AxisValue))

(event Input|AxisEvents|InputAxisAirRoll
  (params (AxisValue :type Float%20%28single-precision%29))
  ;[1 1 1] Input
  (Class|RTuneVehicle|SetAirRollInput (* AxisValue -1.0)))

(event Input|AxisEvents|InputAxisAirYaw
  (params (AxisValue :type Float%20%28single-precision%29))
  ;[1 1 1] Input
  (Class|RTuneVehicle|SetAirYawInput AxisValue))

(fn ConstructionScript
  (bind _front_wheel_meshes (Variables|Settings|GetFront%20Wheel%20Meshes))
  (bind _front_wheel_meshes_2 (Variables|Settings|GetFront%20Wheel%20Meshes))
  (Variables|/Script/RTune.SuspensionComponent|SetWheelMesh (Variables|Default|GetPhysics%20FR) _front_wheel_meshes)
  (Components|StaticMesh|SetStaticMesh (Variables|Default|GetWheel%20FR) _front_wheel_meshes)
  (Variables|/Script/RTune.SuspensionComponent|SetWheelMesh (Variables|Default|GetPhysisc%20FL) _front_wheel_meshes_2)
  (Components|StaticMesh|SetStaticMesh (Variables|Default|GetWheel%20FL) _front_wheel_meshes_2)
  (Transformation|SetRelativeLocation (Variables|Default|GetPhysisc%20FL) (Variables|/Script/Engine.SceneComponent|GetRelativeLocation (Variables|Default|GetSuspension%20FL_Anim)) false false)
  (Transformation|SetRelativeLocation (Variables|Default|GetPhysics%20FR) (Variables|/Script/Engine.SceneComponent|GetRelativeLocation (Variables|Default|GetSuspension%20FR_Anim)) false false))